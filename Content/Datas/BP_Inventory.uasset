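; BP_Inventory holds a slot-based item inventory, storing a name and count per slot.
; Adding stacks onto a matching slot or fills the first empty one, without checking that one exists.
; Removing decrements the count by one and clears the slot at zero, printing a message if the item is absent.
; A linear Find bounded by MaxNbSlot drives both, with "None" marking empty slots, which IsInventoryFull also scans for.
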(event Custom|RemoveFromInventory
  (params (itemName :type Name))
  (bind _inventory (Variables|Default|GetInventory))
  (bind (_index _find) (CallFunction|Find itemName))
  (if _find
    (if (<= (- (.number (Utilities|Array|Get(acopy) _inventory _index)) 1) 0)
      (Utilities|Array|SetArrayElem _inventory _index (Utilities|Struct|MakeDS_InventoryFish "None" 0))
      (else
        (Utilities|Array|SetArrayElem _inventory _index (Utilities|Struct|MakeDS_InventoryFish (.name (Utilities|Array|Get(acopy) _inventory _index)) (- (.number (Utilities|Array|Get(acopy) _inventory _index)) 1)))))
    (else
      (Development|PrintString "Item doesn't exist in inventory" true true "(R=1.000000,G=0.000000,B=0.000000,A=1.000000)" 1e+01))))

(event Custom|AddMultipleToInventory
  (params (ItemName :type Name) (NbToAdd :type Integer))
  (bind _inventory (Variables|Default|GetInventory))
  (bind (_index _find) (CallFunction|Find ItemName))
  (if _find
    (Utilities|Array|SetArrayElem _inventory _index (Utilities|Struct|MakeDS_InventoryFish (.name (Utilities|Array|Get(acopy) _inventory _index)) (+ NbToAdd (.number (Utilities|Array|Get(acopy) _inventory _index)))))
    (else
      (bind _index_2 (CallFunction|FindFirstEmpty))
      (Utilities|Array|SetArrayElem (Variables|Default|GetInventory) _index_2 (Utilities|Struct|MakeDS_InventoryFish ItemName NbToAdd)))))

(fn ConstructionScript)

(fn Find
  (params (Name :type Name))
  (bind (_array_element _array_index) (Utilities|Array|ForEachLoopwithBreak (Variables|Default|GetInventory) :!label _label)
    (:LoopBody
      (if (<= _array_index (Variables|Default|GetMaxNbSlot))
        (if (== (.name _array_element) Name)
          (LocalVariables|SetNewLocalVar _array_index)
          (goto _label Break))
        (else
          (goto _label Break))))
    (:Completed
      (return (LocalVariables|GetNewLocalVar) (!= (LocalVariables|GetNewLocalVar) -1)))))

(fn FindFirstEmpty
  (bind (_index _find) (CallFunction|Find "None"))
  (return _index _find))

(fn IsInventoryFull
  (bind _array_element (Utilities|Array|ForEachLoopwithBreak (Variables|Default|GetInventory) :!label _label)
    (:LoopBody
      (if (== (.name _array_element) "None")
        (LocalVariables|SetNewLocalVar false)
        (goto _label Break)))
    (:Completed
      (return (LocalVariables|GetNewLocalVar)))))