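; BP_RadioLure is a radio device whose wave amplitude and frequency are tuned with the IA_Move input.
; The Y and X axes accumulate into clamped amplitude and frequency values, which drive a dynamic material on the screen, with only amplitude normalized.
; UpdateText shows both values on a text render and forwards them to the GameInstance, also running from the construction script.
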(event Input|EnhancedActionEvents|EnhancedInputActionIA_Move
  (params (ActionValue :type Vector%202D%20Structure) (ElapsedSeconds :type Float%20%28double-precision%29) (TriggeredSeconds :type Float%20%28double-precision%29) (InputAction :type Input%20Action%20Object%20Reference :default "/Game/Input/Actions/IA_Move.IA_Move"))
  (bind _wavematerial (Variables|Default|GetwaveMaterial))
  (Utilities|FlowControl|Sequence
    (:then_0
      (bind _output_get (Variables|Default|SetAmplitude (Math|Float|Clamp(Float) (+ (.y ActionValue) (Variables|Default|GetAmplitude)) 0.0 1e+02)))
      (Rendering|Material|SetScalarParameterValue _wavematerial "Amplitude" (/ _output_get 1e+02) :!class /Script/Engine.MaterialInstanceDynamic))
    (:then_1
      (bind _output_get_2 (Variables|Default|SetFrequency (Math|Float|Clamp(Float) (+ (.x ActionValue) (Variables|Default|GetFrequency)) 0.0 1e+02)))
      (Rendering|Material|SetScalarParameterValue _wavematerial "Frequency" _output_get_2 :!class /Script/Engine.MaterialInstanceDynamic)
      (CallFunction|UpdateText))))

(fn ConstructionScript
  (bind _screen (Variables|Default|GetScreen))
  (|CallParentFunction)
  (bind _returnvalue (Rendering|Material|CreateDynamicMaterialInstance _screen 0 (Rendering|Material|GetMaterial _screen 0) "None" :!class /Script/Engine.PrimitiveComponent))
  (bind _output_get (Variables|Default|SetwaveMaterial _returnvalue))
  (Rendering|Material|SetScalarParameterValue _output_get "Amplitude" 0.0 :!class /Script/Engine.MaterialInstanceDynamic)
  (Rendering|Material|SetScalarParameterValue _output_get "Frequency" 0.0 :!class /Script/Engine.MaterialInstanceDynamic)
  (CallFunction|UpdateText))

(fn UpdateText
  (Rendering|Components|TextRender|SetText (Variables|Default|GetTextRender) (Utilities|Text|ToText(String) (Utilities|String|Append "A: " (Utilities|String|ToString(Float) (Variables|Default|GetAmplitude)) " / 100 ; F: " (Utilities|String|ToString(Float) (Variables|Default|GetFrequency)) " / 100")))
  (Default|ChangeFrequencyandAmplitude (Variables|Default|GetGameInstance) (Variables|Default|GetFrequency) (Variables|Default|GetAmplitude)))