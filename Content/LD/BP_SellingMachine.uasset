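; BP_SellingMachine is a machine that converts fished fish into money.
; When its Possess event fires, it gathers the BP_FishedFish actors overlapping its Box component.
; For each fish it adds the fish's price to the money held through the GameInstance, destroys the fish and prints a debug message.
; The construction script only calls its parent.
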(event EventPossess
  (params (Controller :type BP%20First%20Person%20Character%20Object%20Reference))
  (for _array_element (Collision|GetOverlappingActors (Variables|Default|GetBox) "/Game/Fish/BP_FishedFish.BP_FishedFish_C" :!class /Script/Engine.PrimitiveComponent)
    (bind _asbp_fished_fish (Utilities|Casting|CastToBP_FishedFish _array_element))
    (Default|AddMoney (Variables|Default|GetGameInstance) (Variables|/Game/Fish/BP_FishedFish.BP_FishedFish_C|GetFishPrice _asbp_fished_fish))
    (Actor|DestroyActor _asbp_fished_fish)
    (Development|PrintString "Create money from fish")))

(fn ConstructionScript
  (|CallParentFunction))