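; BP_BaitMachine is a machine that turns fished fish into bait.
; When its Possess event fires, it finds every BP_FishedFish overlapping its Box.
; Each fish adds bait to the GameInstance according to its FishType, with bigger fish giving more, then is destroyed and a message is printed.
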(event EventPossess
  (params (Controller :type BP%20First%20Person%20Character%20Object%20Reference))
  (bind _gameinstance (Variables|Default|GetGameInstance))
  (for _array_element (Collision|GetOverlappingActors (Variables|Default|GetBox) "/Game/Fish/BP_FishedFish.BP_FishedFish_C" :!class /Script/Engine.PrimitiveComponent)
    (bind _asbp_fished_fish (Utilities|Casting|CastToBP_FishedFish _array_element))
    (switch Utilities|FlowControl|Switch|SwitchonEnum_FishType (Variables|/Game/Fish/BP_FishedFish.BP_FishedFish_C|GetFishType _asbp_fished_fish)
      (:NewEnumerator0
        (Default|AddBait _gameinstance 1))
      (:NewEnumerator1
        (Default|AddBait _gameinstance 2))
      (:NewEnumerator2
        (Default|AddBait _gameinstance 3)))
    (Actor|DestroyActor _asbp_fished_fish)
    (Development|PrintString "Create bait from fish")))

(fn ConstructionScript
  (|CallParentFunction))