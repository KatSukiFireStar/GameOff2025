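; BP_SkillTree is a possessable tool actor that opens and closes the skill tree screen.
; On BeginPlay it creates the WBP_SkillTree widget and adds it to the viewport hidden.
; Possessing the tool shows the widget, enables the mouse cursor with Game and UI input, and asks the GameInstance to reload the tree.
; Unpossessing restores game-only input, hides the widget and reloads the UI.
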(event EventBeginPlay
  (|CallParentFunction)
  (bind _returnvalue (UserInterface|CreateWidget "/Game/LD/SkillTree/WBP_SkillTree.WBP_SkillTree_C"))
  (bind _output_get (Variables|Default|SetWidget%20Skill%20Tree _returnvalue))
  (UserInterface|Viewport|AddtoViewport _output_get 0)
  (Variables|/Script/UMG.Widget|SetVisibility _output_get "Hidden"))

(fn ConstructionScript
  (|CallParentFunction))

(fn PossessTool
  (params (CharacterController :type BP%20First%20Person%20Character%20Object%20Reference))
  (bind _returnvalue (Game|GetPlayerController 0))
  (|CallParentFunction CharacterController)
  (Input|SetInputModeGameandUI _returnvalue 0 "LockAlways" false false)
  (Variables|/Script/Engine.PlayerController|SetbShowMouseCursor _returnvalue true)
  (Variables|/Script/UMG.Widget|SetVisibility (Variables|Default|GetWidget%20Skill%20Tree) "Visible")
  (Default|CallReloadTree (Variables|Default|GetGameInstance)))

(fn UnpossessTool
  (bind _returnvalue (Game|GetPlayerController 0))
  (|CallParentFunction)
  (Input|SetInputModeGameOnly _returnvalue false)
  (Variables|/Script/Engine.PlayerController|SetbShowMouseCursor _returnvalue false)
  (Variables|/Script/UMG.Widget|SetVisibility (Variables|Default|GetWidget%20Skill%20Tree) "Hidden")
  (Default|CallReloadUI (Variables|Default|GetGameInstance)))