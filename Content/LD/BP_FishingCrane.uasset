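; BP_FishingCrane is a controllable fishing crane with yaw and clamped camera pitch, used to catch BP_Fish.
; Interaction toggles a timeline that lowers or reverses the line, driving the physics constraint's linear limit and cable length together.
; LureZone overlaps start and stop luring fish toward it.
; HookZone catches one fish and attaches it to the hook, blocking further lowering while that fish stays valid.
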(event OnComponentBeginOverlap(LureZone)
  (params (OverlappedComponent :type Primitive%20Component%20Object%20Reference) (OtherActor :type Actor%20Object%20Reference) (OtherComp :type Primitive%20Component%20Object%20Reference) (OtherBodyIndex :type Integer) (bFromSweep :type Boolean) (SweepResult :type Hit%20Result%20Structure%20%28by%20ref%29))
  (bind _asbp_fish (Utilities|Casting|CastToBP_Fish OtherActor))
  (Default|Lured _asbp_fish (Transformation|GetWorldLocation (Variables|Default|GetLureZone))))

(event OnComponentEndOverlap(LureZone)
  (params (OverlappedComponent :type Primitive%20Component%20Object%20Reference) (OtherActor :type Actor%20Object%20Reference) (OtherComp :type Primitive%20Component%20Object%20Reference) (OtherBodyIndex :type Integer))
  (bind _asbp_fish (Utilities|Casting|CastToBP_Fish OtherActor))
  (Default|StopLured _asbp_fish))

(event OnComponentBeginOverlap(HookZone)
  (params (OverlappedComponent :type Primitive%20Component%20Object%20Reference) (OtherActor :type Actor%20Object%20Reference) (OtherComp :type Primitive%20Component%20Object%20Reference) (OtherBodyIndex :type Integer) (bFromSweep :type Boolean) (SweepResult :type Hit%20Result%20Structure%20%28by%20ref%29))
  (Utilities|IsValid (Variables|Default|GetFish)
    (:Is%20Not%20Valid
      (bind _asbp_fish (Utilities|Casting|CastToBP_Fish OtherActor))
      (bind _output_get (Variables|Default|SetFish _asbp_fish))
      (Default|Fished _output_get)
      (Transformation|AttachComponentToComponent _asbp_fish (Variables|Default|GetHook) "None" "KeepWorld" "KeepWorld" "KeepWorld" true))))

(event EventInteractionEvent
  (if (not (Variables|Default|GetisLoweringLine))
    (Utilities|IsValid (Variables|Default|GetFish)
      (:Is%20Not%20Valid
        (if (Variables|Default|GetisUp)
          (Variables|Default|SetisUp false))
        (Variables|Default|SetisLoweringLine true)
        (bind _alpha (Timeline|LowerLine Play)
          (:Update
            (Class|PhysicsConstraintComponent|SetLinearXLimit (Variables|Default|GetPhysicsConstraint) "LCM_Limited" (+ (* _alpha 9e+02) 1e+01))
            (Variables|/Script/CableComponent.CableComponent|SetCableLength (Variables|Default|GetCable) (+ (* _alpha 9e+02) 1e+01)))
          (:Finished
            (if (not (Variables|Default|GetisLoweringLine))
              (Variables|Default|SetisUp true))))))
    (else
      (Variables|Default|SetisLoweringLine false)
      (Timeline|LowerLine Reverse))))

(fn ConstructionScript
  (|CallParentFunction))

(fn Move
  (params (Xaxis :type Float%20%28single-precision%29) (Yaxis :type Float%20%28double-precision%29))
  (bind _camera (Variables|Default|GetCamera))
  (bind _relativerotation (Variables|/Script/Engine.SceneComponent|GetRelativeRotation _camera))
  (Pawn|Input|AddControllerYawInput (* Xaxis 0.05))
  (Transformation|SetRelativeRotation _camera (Math|Rotator|MakeRotator (.roll _relativerotation) (Math|Float|Clamp(Float) (+ (.pitch _relativerotation) (* Yaxis 0.5)) -45.0 45.0) (.yaw _relativerotation)) false false))