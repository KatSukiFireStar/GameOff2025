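; Fishing net actor that lures little fish, tallies those that touch it and hands the catch to the player's inventory on interaction.
; LureZone overlaps start and stop the lure on little BP_Fish, drawing them toward the zone's location.
; Box overlaps count little fish by name in the FishInNet map.
; InteractionEvent moves each tally into the GameInstance inventory and clears it, stopping when the inventory is full.
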(event OnComponentBeginOverlap(Box)
  (params (OverlappedComponent :type Primitive%20Component%20Object%20Reference) (OtherActor :type Actor%20Object%20Reference) (OtherComp :type Primitive%20Component%20Object%20Reference) (OtherBodyIndex :type Integer) (bFromSweep :type Boolean) (SweepResult :type Hit%20Result%20Structure%20%28by%20ref%29))
  (bind _fishinnet (Variables|Default|GetFishInNet))
  (bind _asbp_fish (Utilities|Casting|CastToBP_Fish OtherActor))
  (switch Utilities|FlowControl|Switch|SwitchonEnum_FishType (Variables|/Game/Fish/BP_Fish.BP_Fish_C|GetfishType _asbp_fish)
    (:NewEnumerator0
      (if (.ReturnValue (Utilities|Map|Find _fishinnet (Variables|/Game/Fish/BP_Fish.BP_Fish_C|GetfishName _asbp_fish)))
        (bind _result (Math|Integer|IncrementInt (.Value (Utilities|Map|Find _fishinnet (Variables|/Game/Fish/BP_Fish.BP_Fish_C|GetfishName _asbp_fish))))
          (:%20%20
            (Utilities|Map|Add _fishinnet (Variables|/Game/Fish/BP_Fish.BP_Fish_C|GetfishName _asbp_fish) _result)))
        (else
          (Utilities|Map|Add _fishinnet (Variables|/Game/Fish/BP_Fish.BP_Fish_C|GetfishName _asbp_fish) 1))))))

(event OnComponentBeginOverlap(LureZone)
  (params (OverlappedComponent :type Primitive%20Component%20Object%20Reference) (OtherActor :type Actor%20Object%20Reference) (OtherComp :type Primitive%20Component%20Object%20Reference) (OtherBodyIndex :type Integer) (bFromSweep :type Boolean) (SweepResult :type Hit%20Result%20Structure%20%28by%20ref%29))
  (bind _asbp_fish (Utilities|Casting|CastToBP_Fish OtherActor))
  (if (Utilities|Enum|Equal(Enum) (Variables|/Game/Fish/BP_Fish.BP_Fish_C|GetfishType _asbp_fish) "NewEnumerator0")
    (Default|Lured _asbp_fish (Transformation|GetWorldLocation (Variables|Default|GetLureZone)))))

(event OnComponentEndOverlap(LureZone)
  (params (OverlappedComponent :type Primitive%20Component%20Object%20Reference) (OtherActor :type Actor%20Object%20Reference) (OtherComp :type Primitive%20Component%20Object%20Reference) (OtherBodyIndex :type Integer))
  (bind _asbp_fish (Utilities|Casting|CastToBP_Fish OtherActor))
  (if (Utilities|Enum|Equal(Enum) (Variables|/Game/Fish/BP_Fish.BP_Fish_C|GetfishType _asbp_fish) "NewEnumerator0")
    (Default|StopLured _asbp_fish)))

(event EventBeginPlay
  (|CallParentFunction) ; This node is disabled and will not be called.\nDrag off pins to build functionality.
)

(event EventInteractionEvent
  (bind _fishinnet (Variables|Default|GetFishInNet))
  (bind _gameinstance (Variables|Default|GetGameInstance))
  (bind _keys (Utilities|Map|Keys _fishinnet))
  (bind _array_element (Utilities|Array|ForEachLoopwithBreak _keys :!label _label)
    (:LoopBody
      (bind _isfull (Default|IsInventoryFull _gameinstance))
      (if _isfull
        (goto _label Break)
        (else
          (Default|AddMultipletoInventory _gameinstance _array_element (.Value (Utilities|Map|Find _fishinnet _array_element)))
          (Utilities|Map|Remove (Variables|Default|GetFishInNet) _array_element))))))

(fn ConstructionScript
  (|CallParentFunction))