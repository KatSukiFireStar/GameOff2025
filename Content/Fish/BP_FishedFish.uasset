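; BP_FishedFish is a fish actor for a fishing mechanic, representing a fish that can be thrown.
; On BeginPlay it looks up FishName in the DT_Fishes data table to set its type and sell price, printing an error if the row is missing.
; ThrowFish detaches it from its parent, enables physics on the skeletal mesh and applies an impulse along the given direction, scaled by ThrowForce.
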(event Custom|ThrowFish
  (params (Direction :type Vector))
  (bind _skeletalmesh (Variables|Default|GetSkeletalMesh))
  (Transformation|DetachFromActor "KeepWorld" "KeepWorld" "KeepWorld")
  (Physics|SetSimulatePhysics _skeletalmesh true)
  (Physics|AddImpulse _skeletalmesh (* Direction (Variables|Default|GetThrowForce)) "None" false))

(event EventBeginPlay
  (CallFunction|SetFishData))

(fn ConstructionScript)

(fn SetFishData
  (bind _returnvalue (Utilities|GetDataTableRow "/Game/Datas/DT_Fishes.DT_Fishes" (Variables|Default|GetfishName))
    (:then
      (Variables|Default|SetFishType (.FishType (Utilities|Struct|BreakDS_Fish _returnvalue)))
      (Variables|Default|SetFishPrice (.SellValue (Utilities|Struct|BreakDS_Fish _returnvalue))))
    (:RowNotFound
      (Development|PrintString "Fish does not exist" true true "(R=1.000000,G=0.011208,B=0.000000,A=1.000000)"))))