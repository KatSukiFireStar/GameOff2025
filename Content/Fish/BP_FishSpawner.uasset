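; Spawner actor that populates the level with fish matching the game instance's current Amplitude and Frequency.
; It binds to the GI_FishGame spawn event and fires it repeatedly after a short startup delay for the initial population.
; Each spawn picks a random class from DT_Fishes rows whose ranges contain both values.
; Fish spawn at random navigable points around the spawner, at its height, and attach to it for scene-tree visibility.
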(event Custom|Spawn%20Fish
  (bind (_fishtospawn _isempty) (CallFunction|GetFishtoSpawn))
  (if (not _isempty)
    (CallFunction|SpawnFish _fishtospawn)))

(event EventBeginPlay
  (bind _asgi_fish_game (Utilities|Casting|CastToGI_FishGame (Game|GetGameInstance)))
  (bind _output_get (Variables|Default|SetGameInstance _asgi_fish_game))
  (EventDispatchers|BindEventtoSpawnNewFish _asgi_fish_game (delegate Custom|Spawn%20Fish))
  (Utilities|FlowControl|Delay 0.2)
  (for _index (range 1 (Variables|Default|GetNbFishStart))
    (Default|CallSpawnNewFish _output_get)))

(fn ConstructionScript)

(fn SpawnFish
  (params (Fish :type BP%20Fish%20Class%20Reference))
  (bind (_randomlocation _returnvalue) (Class|NavigationSystemV1|GetRandomLocationinNavigableRadius (Transformation|GetWorldLocation (Variables|Default|GetDefaultSceneRoot)) 2.5e+03 0 0))
  (if _returnvalue
    (bind _returnvalue_2 (Game|SpawnActorfromClass Fish (Math|Transform|MakeTransform (Math|Vector|MakeVector (.x _randomlocation) (.y _randomlocation) (.z (Transformation|GetWorldLocation (Variables|Default|GetDefaultSceneRoot)))) "0, 0, 0" "1.000000,1.000000,1.000000") "AdjustIfPossibleButAlwaysSpawn" "MultiplyWithRoot" 0 0))
    (Utilities|IsValid _returnvalue_2
      (:Is%20Valid
        ;[0.15 0.15 0.15 0.5] Do this for visibility in scene tree
        (Transformation|AttachActorToActor _returnvalue_2 self "None" "KeepWorld" "KeepWorld" "KeepWorld" true)))))

(fn GetFishtoSpawn
  (bind _spawnablefish (LocalVariables|GetSpawnableFish))
  (bind _gameinstance (Variables|Default|GetGameInstance))
  (bind _returnvalue (Utilities|Set|Length _spawnablefish))
  (bind _outrownames (DataTable|GetDataTableRowNames "/Game/Datas/DT_Fishes.DT_Fishes"))
  (for _array_element _outrownames
    (bind _returnvalue_2 (Utilities|GetDataTableRow "/Game/Datas/DT_Fishes.DT_Fishes" _array_element)
      (:then
        (bind _isinbound (CallFunction|CheckAmplitudeandFrequency (.amplitudemin _returnvalue_2) (.amplitudemax _returnvalue_2) (Variables|/Game/GI_FishGame.GI_FishGame_C|GetAmplitude _gameinstance) (.frequencymin _returnvalue_2) (.frequencymax _returnvalue_2) (Variables|/Game/GI_FishGame.GI_FishGame_C|GetFrequency _gameinstance)))
        (if _isinbound
          (Utilities|Set|Add (LocalVariables|GetSpawnableFish) (.fishbp _returnvalue_2))))))
  (if (> _returnvalue 0)
    (return (Utilities|Set|GetItemByIndex _spawnablefish (Math|Random|RandomIntegerinRange 0 (- _returnvalue 1))) false)
    (else
      (return "/Game/Fish/BP_Fish.BP_Fish_C" true))))

(fn CheckAmplitudeandFrequency
  (params (MinAmplitude :type Float%20%28double-precision%29) (MaxAmplitude :type Float%20%28double-precision%29) (Amplitude :type Float%20%28double-precision%29) (MinFrequency :type Float%20%28double-precision%29) (MaxFrequency :type Float%20%28double-precision%29) (Frequency :type Float%20%28double-precision%29))
  (return (and (and (<= Amplitude MaxAmplitude) (>= Amplitude MinAmplitude)) (and (<= Frequency MaxFrequency) (>= Frequency MinFrequency)))))